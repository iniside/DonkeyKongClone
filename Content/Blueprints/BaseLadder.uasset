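; Base ladder Blueprint for a side-scroller, with a LadderVolume component and a DropLocationEnd offset, but no active logic.
; The LadderVolume end-overlap event is empty, and the construction script does nothing.
; Two identical disconnected chains would cast to SideScrollerCharacter, teleport it to the actor's location plus DropLocationEnd, restore Walking movement and clear IsClimbing.
; Neither chain is triggered, so this dismount behavior never runs.
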(event `self.ReceiveBeginPlay`)

(event `self.ReceiveActorBeginOverlap`
  (params (OtherActor :type "Actor Object Reference")))

(event `self.ReceiveTick`
  (params (DeltaSeconds :type "Float (single-precision)")))

(event `self.LadderVolume.OnComponentEndOverlap`
  (params (OtherActor :type "Actor Object Reference") (OtherComp :type "PrimitiveComponent Object Reference") (OtherBodyIndex :type Integer)))

(fn `UserConstructionScript`)