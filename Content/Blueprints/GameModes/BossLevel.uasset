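; BossLevel, filed under GameModes, builds the boss level's HUD for one or two players.
; After the parent BeginPlay, it creates a collapsed player-died widget and a MasterWidget whose slots receive per-player level score, total score and lives widgets.
; Player 2's widgets are added only when DKGameInstance reports more than one player.
; On Destroyed, it removes all these widgets from their parents.
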(event `self.ReceiveDestroyed`
  (`Widget.RemoveFromParent` (`self.PlayerDiedWid`))
  (`Widget.RemoveFromParent` (`self.BaseScoreWidget`))
  (`Widget.RemoveFromParent` (`self.TotalscoreWidget`))
  (`Widget.RemoveFromParent` (`self.PlayerLivesWidget`))
  (`Widget.RemoveFromParent` (`self.P2_BaseScoreWidget`))
  (`Widget.RemoveFromParent` (`self.P2_TotalscoreWidget`))
  (`Widget.RemoveFromParent` (`self.P2_PlayerLivesWidget`))
  (`Widget.RemoveFromParent` (`self.MasterWidget`)))

(event `self.ReceiveTick`
  (params (DeltaSeconds :type "Float (single-precision)")))

(event `self.ReceiveBeginPlay`
  (`parent.ReceiveBeginPlay`)
  (`|ExecutionSequence`
    (:`then_0`
      (bind _returnvalue (`|CreateWidget` "/Game/UI/Menus/PlayedDiedWidget.PlayedDiedWidget_C"))
      (bind _output_get (set `self.PlayerDiedWid` _returnvalue))
      (`UserWidget.AddToViewport` _output_get 0)
      (`Widget.SetVisibility` _output_get "Collapsed"))
    (:`then_1`
      (`/Engine/EditorBlueprintResources/StandardMacros.IsValid` (`self.MasterWidget`)
        (:`Is Valid`
          _)
        (:`Is Not Valid`
          (bind _returnvalue_2 (`|CreateWidget` "/Game/UI/MasterWidget.MasterWidget_C"))
          (set `self.MasterWidget` _returnvalue_2)))
      (`|ExecutionSequence`
        (:`then_0`
          (`UserWidget.AddToViewport` (`self.MasterWidget`) 0))
        (:`then_1`
          ;[1 1 1] Player 1 Hud
          (bind _returnvalue_3 (`|CreateWidget` "/Game/UI/BaseScore.BaseScore_C"))
          (bind _output_get_2 (set `self.BaseScoreWidget` _returnvalue_3))
          (`PanelWidget.AddChild` (`/Game/UI/MasterWidget.LevelScoreBase` (`self.MasterWidget`)) _output_get_2))
        (:`then_2`
          (bind _returnvalue_4 (`|CreateWidget` "/Game/UI/TotalScoreWidget.TotalScoreWidget_C"))
          (bind _output_get_3 (set `self.TotalscoreWidget` _returnvalue_4))
          (`PanelWidget.AddChild` (`/Game/UI/MasterWidget.TotalScore` (`self.MasterWidget`)) _output_get_3))
        (:`then_3`
          (bind _returnvalue_5 (`|CreateWidget` "/Game/UI/PlayerLivesWidget.PlayerLivesWidget_C"))
          (bind _output_get_4 (set `self.PlayerLivesWidget` _returnvalue_5))
          (`PanelWidget.AddChild` (`/Game/UI/MasterWidget.PlayerLives` (`self.MasterWidget`)) _output_get_4))
        (:`then_4`
          (bind _asdkgame_instance (cast `DKGameInstance` (`GameplayStatics.GetGameInstance`)))
          (if (> (`DKGameInstance.PlayerNumber` _asdkgame_instance) 1)
            (`|ExecutionSequence`
              (:`then_0`
                ;[1 1 1] Player 2 Hud
                (bind _returnvalue_6 (`|CreateWidget` "/Game/UI/BaseScore.BaseScore_C" null 1))
                (bind _output_get_5 (set `self.P2_BaseScoreWidget` _returnvalue_6))
                (`PanelWidget.AddChild` (`/Game/UI/MasterWidget.P2_LevelScoreBase` (`self.MasterWidget`)) _output_get_5))
              (:`then_1`
                (bind _returnvalue_7 (`|CreateWidget` "/Game/UI/TotalScoreWidget.TotalScoreWidget_C" null 1))
                (bind _output_get_6 (set `self.P2_TotalscoreWidget` _returnvalue_7))
                (`PanelWidget.AddChild` (`/Game/UI/MasterWidget.P2_TotalScore` (`self.MasterWidget`)) _output_get_6))
              (:`then_2`
                (bind _returnvalue_8 (`|CreateWidget` "/Game/UI/PlayerLivesWidget.PlayerLivesWidget_C" null 1))
                (bind _output_get_7 (set `self.P2_PlayerLivesWidget` _returnvalue_8))
                (`PanelWidget.AddChild` (`/Game/UI/MasterWidget.P2_PlayerLives` (`self.MasterWidget`)) _output_get_7)))))))))

(fn `UserConstructionScript`)