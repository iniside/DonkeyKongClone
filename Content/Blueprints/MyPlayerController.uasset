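; Player controller that owns the player's HUD widgets: floating score popups, a respawn screen and a game over screen.
; BeginPlay creates all widgets collapsed, including a fixed pool of floating score widgets, and Destroyed removes them.
; Game over and spectate events reveal their screens, while OnScoreAdded reuses the first collapsed pooled widget, passing it the location and score.
; ShowFloatingScore holds an unconnected copy of that pool logic and does nothing.
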(event `self.ReceiveDestroyed`
  (bind _floatnigscorewidgets (`self.FloatnigScoreWidgets`))
  (`Widget.RemoveFromParent` (`self.RespawnScreenWidget`))
  (`Widget.RemoveFromParent` (`self.GameOverWidget`))
  (for _array_element _floatnigscorewidgets
    (`Widget.RemoveFromParent` _array_element))
  (`KismetArrayLibrary.Array_Clear` _floatnigscorewidgets))

(event `self.ReceiveBeginPlay`
  (`|ExecutionSequence`
    (:`then_0`
      (for _ (range 11)
        (bind _returnvalue (`|CreateWidget` "/Game/UI/FloatingScoreWidget.FloatingScoreWidget_C"))
        (`UserWidget.AddToViewport` _returnvalue 0)
        (`Widget.SetVisibility` _returnvalue "Collapsed")
        (`KismetArrayLibrary.Array_Add` (`self.FloatnigScoreWidgets`) _returnvalue)))
    (:`then_1`
      (bind _returnvalue_2 (`|CreateWidget` "/Game/UI/Menus/RespawnScreen.RespawnScreen_C"))
      (bind _output_get (set `self.RespawnScreenWidget` _returnvalue_2))
      (`UserWidget.AddToViewport` _output_get 0)
      (`Widget.SetVisibility` _output_get "Collapsed"))
    (:`then_2`
      (bind _returnvalue_3 (`|CreateWidget` "/Game/UI/Menus/GameOverWidget.GameOverWidget_C"))
      (bind _output_get_2 (set `self.GameOverWidget` _returnvalue_3))
      (`UserWidget.AddToViewport` _output_get_2 0)
      (`Widget.SetVisibility` _output_get_2 "Collapsed"))))

(event `self.OnGameOver`
  (`Widget.SetVisibility` (`self.GameOverWidget`) "Visible"))

(event `self.OnStartSpectate`
  (`Widget.SetVisibility` (`self.RespawnScreenWidget`) "Visible"))

(event `self.ReceiveTick`
  (params (DeltaSeconds :type "Float (single-precision)")))

(event `self.OnScoreAdded`
  (params (PlayerIndex :type Integer) (TargetLocation :type "Object.Vector Structure (by ref)") (Score :type Integer))
  (for _array_element (`self.FloatnigScoreWidgets`)
    (switch `ESlateVisibility` (`Widget.GetVisibility` _array_element)
      (:`Collapsed`
        (set `/Game/UI/FloatingScoreWidget.TargetLocation` TargetLocation _array_element)
        (set `/Game/UI/FloatingScoreWidget.Score` Score _array_element)
        (`/Game/UI/FloatingScoreWidget.ShowWidget` _array_element)
        (break)))))

(fn `ShowFloatingScore`
  (params (TargetLocation :type "Object.Vector Structure" :default (0.0 0.0 0.0)) (Score :type Integer :default 0)))

(fn `UserConstructionScript`)