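; RollingBarrel is an actor that rolls along platforms on the Y axis, drops off their edges and reverses direction after each fall.
; Each Tick moves it without sweep, sets RotatingMovement's spin and traces down from its trailing side for WorldStatic ground.
; A hit sets rolling velocity and eases its height onto the surface.
; A miss makes it fall, with ChangeDirection ensuring MoveDirection flips only once per drop.
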(event `self.ReceiveBeginPlay`)

(event `self.ReceiveActorBeginOverlap`
  (params (OtherActor :type "Actor Object Reference")))

(event `self.ReceiveTick`
  (params (DeltaSeconds :type "Float (single-precision)"))
  (bind _returnvalue (`self.K2_GetActorLocation`))
  (bind _returnvalue_2 (+ (`self.K2_GetActorLocation`) (`self.TraceDirection`)))
  (`self.K2_AddActorWorldOffset` (* (`self.Move`) DeltaSeconds))
  (set `RotatingMovementComponent.RotationRate` (`self.RotationRate`) (`self.RotatingMovement`))
  (bind (_outhit _returnvalue_3) (`KismetSystemLibrary.LineTraceSingleForObjects` :`Start` _returnvalue_2 :`End` (+ _returnvalue_2 (* (0.0 0.0 -1.0) 70.0)) :`ObjectTypes` (`|MakeArray` "ObjectTypeQuery1" :!type "EngineTypes.EObjectTypeQuery Enum") :`DrawDebugType` "ForDuration"))
  (if _returnvalue_3
    (if (`self.MoveDirection`)
      (set `self.Move` (0.0 -400.0 0.0))
      (set `self.TraceDirection` (0.0 40.0 0.0))
      (set `self.RotationRate` (struct :`Roll` -180.0))
      (else
        (set `self.Move` (0.0 400.0 0.0))
        (set `self.TraceDirection` (0.0 -40.0 0.0))
        (set `self.RotationRate` (struct :`Roll` 180.0))))
    (set `self.ChangeDirection` true)
    (`self.K2_SetActorLocation` (`KismetMathLibrary.VInterpTo` _returnvalue (`KismetMathLibrary.MakeVector` (.x _returnvalue) (.y _returnvalue) (+ (.z (`.Location` (`GameplayStatics.BreakHitResult` _outhit))) 40.0)) (`GameplayStatics.GetWorldDeltaSeconds`) 5.0))
    (else
      (set `self.Move` (0.0 0.0 -300.0))
      (if (`self.ChangeDirection`)
        (if (`self.MoveDirection`)
          (set `self.MoveDirection` false)
          (else
            (set `self.MoveDirection` true)))
        (set `self.ChangeDirection` false)))))

(fn `UserConstructionScript`)